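; BP_NCharacter is a player character Blueprint that handles basic movement, look and jump input.
; Turn and LookUp axes drive controller yaw and pitch, while Forward and Right move the character along the capsule's forward and right vectors.
; The right mouse button is bound directly as a key event to DetectObjects, whose implementation is outside this graph.
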(event `InputAxis|Turn`
  (params (AxisValue :type "Float (single-precision)"))
  (`self.AddControllerYawInput` AxisValue))

(event `InputAxis|LookUp`
  (params (AxisValue :type "Float (single-precision)"))
  (`self.AddControllerPitchInput` AxisValue))

(event `InputAction|Jump`
  (params (Key :type "Key Structure"))
  (:`Pressed`
    (`self.Jump`)))

(event `InputAxis|Forward`
  (params (AxisValue :type "Float (single-precision)"))
  (`self.AddMovementInput` (`SceneComponent.GetForwardVector` (`self.CapsuleComponent`)) AxisValue))

(event `InputAxis|Right`
  (params (AxisValue :type "Float (single-precision)"))
  (`self.AddMovementInput` (`SceneComponent.GetRightVector` (`self.CapsuleComponent`)) AxisValue))

(event `Key|RightMouseButton`
  (params (Key :type "Key Structure"))
  (:`Pressed`
    (`self.DetectObjects`)))

(fn `UserConstructionScript`)