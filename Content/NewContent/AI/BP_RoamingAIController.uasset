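; AI controller for roaming AI that starts the BT_RoamingAI behavior tree on BeginPlay.
; ClosestPointOutsideRadius randomly samples navigable points until one lies outside a radius around Origin and within Proximity of another point.
; Once the attempt counter exceeds its limit, it falls back to a random navigable point around that other point.
; GetAbilityPosibilities is an empty stub.
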(event `self.ReceiveBeginPlay`
  (`self.RunBehaviorTree` "/Game/NewContent/AI/BT_RoamingAI.BT_RoamingAI"))

(fn `ClosestPointOutsideRadius`
  (params (Origin :type "Vector Structure") (Radius :type "Float (double-precision)") (Accuracy :type "Float (double-precision)") (OtherPoint :type "Vector Structure") (Proximity :type "Float (double-precision)"))
  (returns (ClosestPoint :type "Vector Structure"))
  (locals (Attempts :type "Float (double-precision)") (MaxNumberAttempts :type "Float (double-precision)" :default 1000.0))
  (while true
    (bind _randomlocation (`NavigationSystemV1.K2_GetRandomLocationInNavigableRadius` Origin (+ Radius Accuracy) null null))
    (if (> (`KismetMathLibrary.VSize` (- Origin _randomlocation)) Radius)
      (if (<= (`KismetMathLibrary.VSize` (- OtherPoint _randomlocation)) Proximity)
        (return _randomlocation)
        (else
          _)))
    (if (> (`local.Attempts`) (`local.MaxNumberAttempts`))
      (bind _randomlocation_2 (`NavigationSystemV1.K2_GetRandomLocationInNavigableRadius` OtherPoint Radius null null))
      (return _randomlocation_2)
      (else
        (`/Engine/EditorBlueprintResources/StandardMacros.IncrementFloat` (`local.Attempts`))))))

(fn `GetAbilityPosibilities`
  (params (AvailableAbilities :type "Array of GameplayAbility Class Reference (by ref)"))
  (returns (PosibleActions :type "/Game/NewContent/DataStructures/ST_InteractablePosibilities Structure"))
  (return))

(fn `UserConstructionScript`)