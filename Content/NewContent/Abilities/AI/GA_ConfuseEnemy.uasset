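; GA_ConfuseEnemy is a gameplay ability that distracts an AI target with a hologram decoy of the player.
; After committing, it waits for a Player-tagged gameplay event and checks that the target implements BPI_AbilityAIInteractable.
; It then spawns BP_HologramPlayer at the instigating first-person character's transform and passes it to the target through DecoyEffectMessage.
; The ability ends afterwards or on a failed commit or interface check, but not on a failed cast.
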(event `self.K2_ActivateAbility`
  (bind _returnvalue (`self.K2_CommitAbility`))
  (if _returnvalue
    (bind (_asynctaskproxy _payload) (`AbilityTask_WaitGameplayEvent.WaitGameplayEvent` (struct :`TagName` "Player") null)
      (:`EventReceived`
        (bind (_eventtag _instigator _target) (break `GameplayEventData` _payload))
        (if (`KismetSystemLibrary.DoesImplementInterface` _target "/Game/NewContent/Interfaces/BPI_AbilityAIInteractable.BPI_AbilityAIInteractable_C")
          (bind _asbp_first_person_character (cast `/Game/FirstPerson/Blueprints/BP_FirstPersonCharacter` _instigator))
          (bind _returnvalue_2 (`|SpawnActorFromClass` "/Game/NewContent/Hologram/BP_HologramPlayer.BP_HologramPlayer_C" (`Actor.GetTransform` _asbp_first_person_character) "Undefined" "MultiplyWithRoot" null null))
          (message `/Game/NewContent/Interfaces/BPI_AbilityAIInteractable.DecoyEffect` _target _returnvalue_2)
          (`self.K2_EndAbility`)
          (else
            (`self.K2_EndAbility`)))))
    (else
      (`self.K2_EndAbility`))))