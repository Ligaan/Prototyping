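; BP_NCube is an actor with a Cube component whose custom depth rendering switches off after a short delay.
; While the Reseted flag is true, Tick accumulates delta time in Dt.
; Once Dt passes three seconds, it disables custom depth on the Cube and clears both the flag and the timer.
; Nothing in this graph sets the flag or enables custom depth.
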(event `self.ReceiveTick`
  (params (DeltaSeconds :type "Float (single-precision)"))
  (if (`self.Reseted`)
    (bind _output_get (set `self.dt` (+ DeltaSeconds (`self.dt`))))
    (if (> _output_get 3.0)
      (`PrimitiveComponent.SetRenderCustomDepth` (`self.Cube`) false)
      (set `self.Reseted` false)
      (set `self.dt` 0.0))))

(fn `UserConstructionScript`)