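; BP_Cube is a cube actor that clears a temporary overlay material shortly after being flagged as reset.
; While the Reseted flag is true, Tick accumulates delta time into TimeSinceReset.
; Once three seconds pass, it calls SetOverlayMaterial with no material on the Cube component, then clears the flag and timer.
; Nothing in this Blueprint sets the flag or applies the overlay.
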(event `self.ReceiveTick`
  (params (DeltaSeconds :type "Float (single-precision)"))
  (if (`self.Reseted`)
    (bind _output_get (set `self.TimeSinceReset` (+ DeltaSeconds (`self.TimeSinceReset`))))
    (if (> _output_get 3.0)
      (`MeshComponent.SetOverlayMaterial` (`self.Cube`) null)
      (set `self.Reseted` false)
      (set `self.TimeSinceReset` 0.0))))

(fn `UserConstructionScript`)