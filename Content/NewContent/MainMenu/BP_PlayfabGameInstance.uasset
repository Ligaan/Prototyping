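; Game instance that wraps PlayFab account and multiplayer lobby services for the main menu.
; Init sets the title; sign-up and login open the find-lobby level, with login caching entity and auth context for lobby requests.
; Events create, find, join, get, delete and leave lobbies, building JSON payloads and mostly printing results.
; CloseLobby loops over fetched members before leaving, but RemoveMemberFromLobby is an empty stub with its request disconnected.
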(event `self.ReceiveInit`
  ;[1 1 1] Playfab game settings
  (`PlayFabUtilities.setPlayFabSettings` (`self.GameId`)))

(event `OnRegisterSuccess`
  (params (result :type "ClientRegisterPlayFabUserResult Structure") (customData :type "Object Object Reference"))
  ;[1 1 1] SignUp
  (`GameplayStatics.OpenLevel` "FindLobbyMenu_Level"))

(event `SignUp`
  (params (Usename :type String) (Email :type String) (Password :type String))
  ;[1 1 1] SignUp
  (`PlayFabClientAPI.RegisterPlayFabUser` (make `ClientRegisterPlayFabUserRequest` null Usename Email "" null Password "" false Usename) (delegate `OnRegisterSuccess`) (delegate `OnFail`)))

(event `OnFail`
  (params (error :type "PlayFabError Structure") (customData :type "Object Object Reference"))
  ;[1 1 1] SignUp
  (`KismetSystemLibrary.PrintString` (`KismetStringLibrary.Concat_StrStr` error_ErrorName ":" error_ErrorMessage "(" error_ErrorDetails ")") true true (struct :`R` 1.0 :`G` 0.064383 :`A` 1.0) 60.0))

(event `LogIn`
  (params (Email :type String) (Password :type String))
  ;[1 1 1] Log In
  (`PlayFabClientAPI.LoginWithEmailAddress` (make `ClientLoginWithEmailAddressRequest` null Email null Password) (delegate `OnLogInSuccess`) (`|CreateDelegate` :!event `OnFail`)))

(event `OnLogInSuccess`
  (params (result :type "ClientLoginResult Structure") (customData :type "Object Object Reference"))
  (bind (_entitytoken _inforesultpayload _lastlogintime _newlycreated _playfabid _sessionticket _settingsforuser _treatmentassignment _authenticationcontext) (break `ClientLoginResult` result))
  ;[1 1 1] Log In
  (`GameplayStatics.OpenLevel` "FindLobbyMenu_Level")
  (bind _output_get (set `self.UserToken` _entitytoken))
  (set `self.UserPlayfabId` _playfabid)
  (set `self.Entity` (`PlayFabJsonObject.GetObjectField` _output_get "Entity"))
  (set `self.PlayerAC` _authenticationcontext))

(event `RecoveryEmailSuccess`
  (params (result :type "ClientSendAccountRecoveryEmailResult Structure") (customData :type "Object Object Reference"))
  ;[1 1 1] Account Recovery
  (`KismetSystemLibrary.PrintString` "A recovery email has been sent." true true (struct :`G` 1.0 :`B` 0.044955 :`A` 1.0) 10.0))

(event `ForgotPassword`
  (params (Email :type String))
  ;[1 1 1] Account Recovery
  (`PlayFabClientAPI.SendAccountRecoveryEmail` (make `ClientSendAccountRecoveryEmailRequest` null Email) (delegate `RecoveryEmailSuccess`) (`|CreateDelegate` :!event `OnFail`)))

(event `LobbyCreatedSuccessfully`
  (params (result :type "MultiplayerCreateLobbyResult Structure") (customData :type "Object Object Reference"))
  ;[1 1 1] Create Lobby
  (bind _output_get (set `self.Session` result_ConnectionString))
  (set `self.LobbyId` result_LobbyId)
  (`KismetSystemLibrary.PrintString` _output_get true true (struct :`G` 0.66 :`B` 1.0 :`A` 1.0) 10.0))

(event `CreateMultiplayerLobby`
  ;[1 1 1] Create Lobby
  (bind _output_get (set `self.LobbySearchData` (`PlayFabJsonObject.ConstructJsonObject`)))
  (`PlayFabJsonObject.SetStringField` _output_get "string_key1" "test")
  (bind _output_get_2 (set `self.Temp Json` (`PlayFabJsonObject.ConstructJsonObject`)))
  (`PlayFabJsonObject.SetObjectField` _output_get_2 "MemberEntity" (`self.Entity`))
  (bind _output_get_3 (set `self.Member Type` (`PlayFabJsonObject.ConstructJsonObject`)))
  (`PlayFabJsonObject.SetStringField` _output_get_3 "MemberType" "Server")
  (`PlayFabJsonObject.SetObjectField` _output_get_3 "MemberData" _output_get_2)
  (`PlayFabMultiplayerAPI.CreateLobby` (make `MultiplayerCreateLobbyRequest` "pfenum_Public" null null 2 (`|MakeArray` (`self.Temp Json`)) (`self.Entity`) "pfenum_Manual" (`self.LobbySearchData`) true (`self.PlayerAC`)) (delegate `LobbyCreatedSuccessfully`) (`|CreateDelegate` :!event `OnFail`)))

(event `OnJoiningLobby`
  (params (result :type "MultiplayerJoinLobbyResult Structure") (customData :type "Object Object Reference"))
  ;[1 1 1] Join Lobby
)

(event `JoinLobby`
  (params (ConnectionString :type String))
  ;[1 1 1] Join Lobby
  (`PlayFabMultiplayerAPI.JoinLobby` (make `MultiplayerJoinLobbyRequest` ConnectionString null null (`self.Temp Json`)) (delegate `OnJoiningLobby`) (`|CreateDelegate` :!event `OnFail`)))

(event `ShowLobbies`
  (params (result :type "MultiplayerFindLobbiesResult Structure") (customData :type "Object Object Reference"))
  ;[1 1 1] Find Lobbies
  (for _array_element result_Lobbies
    (`KismetSystemLibrary.PrintString` (`KismetStringLibrary.Conv_ObjectToString` _array_element) true true (struct :`G` 0.66 :`B` 1.0 :`A` 1.0) 10.0)))

(event `FindLobbies`
  ;[1 1 1] Find Lobbies
  (`PlayFabMultiplayerAPI.FindLobbies` (make `MultiplayerFindLobbiesRequest` null "$filter=string_key1 eq test" "" null (`self.PlayerAC`)) (delegate `ShowLobbies`) (`|CreateDelegate` :!event `OnFail`)))

(event `LobbyDeleted`
  (params (result :type "MultiplayerLobbyEmptyResult Structure") (customData :type "Object Object Reference"))
  ;[1 1 1] Delete Lobby
  (`KismetSystemLibrary.PrintString` "Lobby was succesfully deleted!")
  (set `self.LobbyId` ""))

(event `DeleteLobby`
  (bind _lobbyid (`self.LobbyId`))
  ;[1 1 1] Delete Lobby
  (if (`KismetStringLibrary.NotEqual_StrStr` _lobbyid)
    (`PlayFabMultiplayerAPI.DeleteLobby` (make `MultiplayerDeleteLobbyRequest` null _lobbyid (`self.PlayerAC`)) (delegate `LobbyDeleted`) (`|CreateDelegate` :!event `OnFail`))))

(event `LobbyFound`
  (params (result :type "MultiplayerGetLobbyResult Structure") (customData :type "Object Object Reference"))
  ;[1 1 1] GetLobby
  (set `self.LobbyData` (`.Lobby` (break `MultiplayerGetLobbyResult` result)))
  (if (`self.Shutdown`)
    (`self.CloseLobby`)))

(event `GetLobby`
  ;[1 1 1] GetLobby
  (`PlayFabMultiplayerAPI.GetLobby` (make `MultiplayerGetLobbyRequest` null (`self.LobbyId`) (`self.PlayerAC`)) (delegate `LobbyFound`) (`|CreateDelegate` :!event `OnFail`)))

(event `CloseLobby`
  (bind _lobbydata (`self.LobbyData`))
  ;[1 1 1] Close Lobby
  (`/Engine/EditorBlueprintResources/StandardMacros.IsValid` _lobbydata
    (:`Is Valid`
      (bind _returnvalue (`PlayFabJsonObject.GetObjectArrayField` _lobbydata "Members"))
      (for _array_element _returnvalue
        (bind _output_get (set `self.Temp` (`PlayFabJsonObject.ConstructJsonObject`)))
        (`PlayFabJsonObject.SetField` _output_get "MemberEntity" (`PlayFabJsonObject.GetField` _array_element "MemberEnity"))
        (`self.RemoveMemberFromLobby` (`self.Temp`))))
    (:`Is Not Valid`
      _))
  (`self.LeaveLobby`))

(event `OnRemoveMemberSuccess`
  (params (result :type "MultiplayerLobbyEmptyResult Structure") (customData :type "Object Object Reference"))
  ;[1 1 1] Remove Member
  (`KismetSystemLibrary.PrintString` "Member Removed Succesfully" true true (struct :`G` 0.66 :`B` 1.0 :`A` 1.0) 5.0))

(event `RemoveMemberFromLobby`
  (params (NewParam :type "PlayFabJsonObject Object Reference"))
  ;[1 1 1] Remove Member
)

(event `OnLeaveLobbySuccess`
  (params (result :type "MultiplayerLobbyEmptyResult Structure") (customData :type "Object Object Reference"))
  ;[1 1 1] Leave Lobby
  (`KismetSystemLibrary.PrintString` "Leave Lobby Completed" true true (struct :`R` 0.110741 :`G` 1.0 :`A` 1.0)))

(event `LeaveLobby`
  ;[1 1 1] Leave Lobby
  (`PlayFabMultiplayerAPI.LeaveLobby` (make `MultiplayerLeaveLobbyRequest` :`LobbyId` (`self.LobbyId`) :`MemberEntity` (`self.Entity`) :`AuthenticationContext` (`self.PlayerAC`)) (delegate `OnLeaveLobbySuccess`) (`|CreateDelegate` :!event `OnFail`)
    (:`then`
      (set `self.LobbyId` ""))))

(fn `NewFunction`)