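; Player character with first-person-style look, jump and movement along capsule axes, whose gravity switches when it overlaps actors tagged Wall.
; If the wall's inverted up vector differs from current gravity, it teleport-rotates the character by combining its rotation with the wall's forward look-at.
; It then stores that vector as GravityDirection and applies it through UpdateGravityDirection, which casts and caches a custom NewGravityMovementComponent.
; An unconnected controller-input rotation alternative remains in the overlap graph.
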(event `InputAxis|LookUp`
  (params (AxisValue :type "Float (single-precision)"))
  (`self.AddControllerPitchInput` AxisValue))

(event `InputAxis|Turn`
  (params (AxisValue :type "Float (single-precision)"))
  (`self.AddControllerYawInput` AxisValue))

(event `InputAxis|Forward`
  (params (AxisValue :type "Float (single-precision)"))
  (`self.AddMovementInput` (`SceneComponent.GetForwardVector` (`self.CapsuleComponent`)) AxisValue))

(event `InputAxis|Right`
  (params (AxisValue :type "Float (single-precision)"))
  (`self.AddMovementInput` (`SceneComponent.GetRightVector` (`self.CapsuleComponent`)) AxisValue))

(event `InputAction|Jump`
  (params (Key :type "Key Structure"))
  (:`Pressed`
    (`self.Jump`)))

(event `self.ReceiveTick`
  (params (DeltaSeconds :type "Float (single-precision)")))

(event `self.ReceiveActorBeginOverlap`
  (params (OtherActor :type "Actor Object Reference"))
  (bind _returnvalue (`self.K2_GetActorLocation`))
  (bind _returnvalue_2 (* (`self.GetActorUpVector` OtherActor) -1.0))
  (if (and (`self.ActorHasTag` OtherActor "Wall") (!= _returnvalue_2 (`self.Gravity Direction`)))
    (`self.K2_SetActorTransform` (`KismetMathLibrary.MakeTransform` (`self.K2_GetActorLocation`) (`KismetMathLibrary.ComposeRotators` (`self.K2_GetActorRotation`) (`KismetMathLibrary.FindLookAtRotation` _returnvalue (+ _returnvalue (* (`self.GetActorForwardVector` OtherActor) 10.0))))) false true)
    (set `self.Gravity Direction` _returnvalue_2)
    (`self.UpdateGravityDirection`)))

(fn `UpdateGravityDirection`
  (`self.NewGravityMovementComponent`
    (:`then`
      _)
    (:`else`
      (bind _asnew_gravity_movement_component (cast `NewGravityMovementComponent` (`self.CharacterMovement`)))
      (set `self.NewGravityMovementComponent` _asnew_gravity_movement_component)))
  (`CharacterMovementComponent.SetGravityDirection` (`self.CharacterMovement`) (`self.Gravity Direction`)))

(fn `UserConstructionScript`)