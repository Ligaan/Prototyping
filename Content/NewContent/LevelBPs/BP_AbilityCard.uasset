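; BP_AbilityCard is a pickup that grants its stored gameplay ability to the first-person character who overlaps it.
; On BeginPlay, it converts the ability's class name to a number, maps that to a color and sets it on the sphere's dynamic material, also printing the number.
; On overlap, it searches the character's ability list and, only if the ability is absent, adds it and destroys itself.
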(event `self.ReceiveBeginPlay`
  (bind _returnvalue (`StringUtils.StringToNumber` (`KismetSystemLibrary.GetClassDisplayName` (`self.AbilityStored`))))
  (`KismetSystemLibrary.PrintString` (`KismetStringLibrary.Conv_IntToString` _returnvalue))
  (bind _returnvalue_2 (`PrimitiveComponent.CreateDynamicMaterialInstance` (`self.Sphere`) 0 null "None"))
  (`MaterialInstanceDynamic.SetVectorParameterValue` _returnvalue_2 "Color" (`StringUtils.NumberToColor` _returnvalue)))

(event `self.ReceiveActorBeginOverlap`
  (params (OtherActor :type "Actor Object Reference"))
  (bind _asbp_first_person_character (cast `/Game/FirstPerson/Blueprints/BP_FirstPersonCharacter` OtherActor))
  (for _array_element (`DefaultCharacter.GameplayAbilities` _asbp_first_person_character)
    (bind _returnvalue (== _array_element (`self.AbilityStored`)))
    (set `self.NotValid` _returnvalue)
    (if _returnvalue
      (break)))
  (if (not (`self.NotValid`))
    (`/Game/FirstPerson/Blueprints/BP_FirstPersonCharacter.Add Ability` _asbp_first_person_character (`self.AbilityStored`))
    (`self.K2_DestroyActor`)))

(fn `UserConstructionScript`)