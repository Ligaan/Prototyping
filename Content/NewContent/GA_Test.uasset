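; GA_Test is a test Gameplay Ability that pushes a target actor away along the instigator's forward vector.
; On activation it commits, then waits for a single RotateAbility gameplay event, ending immediately if the commit fails.
; The event payload supplies instigator and target, and the target's primitive component receives a large impulse despite the tag's name.
; It prints a debug success or failure message, then ends.
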(event `self.K2_ActivateAbility`
  (bind _returnvalue (`self.K2_CommitAbility`))
  (if _returnvalue
    (bind (_asynctaskproxy _payload) (`AbilityTask_WaitGameplayEvent.WaitGameplayEvent` (struct :`TagName` "RotateAbility") null true)
      (:`EventReceived`
        (bind (_eventtag _instigator _target) (break `GameplayEventData` _payload))
        (bind _returnvalue_2 (`Actor.GetComponentByClass` _target "/Script/Engine.PrimitiveComponent"))
        (if (`KismetSystemLibrary.IsValid` _returnvalue_2)
          (`PrimitiveComponent.AddImpulse` _returnvalue_2 (* (`Actor.GetActorForwardVector` _instigator) 100000.0) "None" false)
          (`KismetSystemLibrary.PrintString` "Hello")
          (else
            (`KismetSystemLibrary.PrintString` "Fail")))
        (`self.K2_EndAbility`)))
    (else
      (`self.K2_EndAbility`))))